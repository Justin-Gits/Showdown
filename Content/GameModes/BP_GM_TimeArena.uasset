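; BP_GM_TimeArena is a game mode Blueprint for the Time Arena mode that spawns player characters.
; SpawnCharacterforPlayer spawns a BP_CHAR_Player at a random entry in Team1PlayerStarts and has the given PlayerController possess it.
; If that array is empty, it logs a message and lazily fills it with every PlayerStart actor in the level, with no team filtering.
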(event EventSpawnCharacterforPlayer
  (params (PlayerController :type PC%20Player%20Object%20Reference))
  (if (> (Utilities|Array|Length (Variables|Default|GetTeam1%20Player%20Starts)) 0)
    _
    (else
      (Development|PrintString "Player Start Array not Initialized, initializing now.")
      (bind _outactors (Actor|GetAllActorsOfClass "/Script/Engine.PlayerStart"))
      (Variables|Default|SetTeam1%20Player%20Starts _outactors)))
  (bind _returnvalue (Game|SpawnActorfromClass "/Game/Characters/BP_CHAR_Player.BP_CHAR_Player_C" (Transformation|GetActorTransform (.OutItem (Utilities|Array|Random (Variables|Default|GetTeam1%20Player%20Starts)))) "Undefined" "MultiplyWithRoot" 0 0))
  (Pawn|Possess PlayerController _returnvalue))

(fn ConstructionScript)